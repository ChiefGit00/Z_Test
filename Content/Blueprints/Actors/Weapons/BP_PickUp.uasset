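; Weapon pickup actor that shows a prompt widget on overlap and gives its weapon type to the player on interact, then destroys itself.
; While BP_Char overlaps the box, a looping timer turns the widget toward the view using control rotation and polls the player's Interact flag.
; SetType swaps the melee, semi-auto or auto mesh, at construction or from Drop, which randomizes the type or leaves it unchanged.
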(event OnComponentBeginOverlap(Box)
  (params (OverlappedComponent :type Primitive%20Component%20Object%20Reference) (OtherActor :type Actor%20Object%20Reference) (OtherComp :type Primitive%20Component%20Object%20Reference) (OtherBodyIndex :type Integer) (bFromSweep :type Boolean) (SweepResult :type Hit%20Result%20Structure%20%28by%20ref%29))
  (bind _asbp_char (Utilities|Casting|CastToBP_Char OtherActor))
  (Variables|Default|SetPlayerPawn _asbp_char)
  (Rendering|SetVisibility (Variables|Default|GetWidget) true false)
  (bind _returnvalue (Utilities|Time|SetTimerbyEvent (delegate Custom|WB_Rotate) 0.01 true))
  (Variables|Default|SetTimer_WBRotate _returnvalue))

(event OnComponentEndOverlap(Box)
  (params (OverlappedComponent :type Primitive%20Component%20Object%20Reference) (OtherActor :type Actor%20Object%20Reference) (OtherComp :type Primitive%20Component%20Object%20Reference) (OtherBodyIndex :type Integer))
  (Utilities|Casting|CastToBP_Char OtherActor)
  (Rendering|SetVisibility (Variables|Default|GetWidget) false false)
  (Utilities|Time|ClearandInvalidateTimerbyHandle (Variables|Default|GetTimer_WBRotate)))

(event Custom|WB_Rotate
  (bind _returnvalue (Game|GetPlayerController 0))
  (bind _returnvalue_2 (Pawn|GetControlRotation _returnvalue :!class /Script/Engine.Controller))
  (Transformation|SetWorldRotation (Variables|Default|GetWidget) (Math|Rotator|MakeRotator (.roll _returnvalue_2) (.pitch _returnvalue_2) (- (.yaw _returnvalue_2) 1.8e+02)) false false)
  (if (Variables|/Game/Blueprints/Game/BP_Char.BP_Char_C|GetbInteract (Variables|Default|GetPlayerPawn))
    (Default|PickUpWeapon (Variables|Default|GetPlayerPawn) (Variables|Default|GetWeaponType))
    (Actor|DestroyActor)))

(event Custom|Drop
  (switch int (Math|Random|RandomIntegerinRange 0 4)
    (:2
      (CallFunction|SetType "NewEnumerator2"))
    (:3
      (CallFunction|SetType "NewEnumerator2"))
    (:4
      (CallFunction|SetType "NewEnumerator3"))))

(event EventTick
  (params (DeltaSeconds :type Float%20%28single-precision%29))
  (Utilities|FlowControl|Gate true))

(fn ConstructionScript
  (CallFunction|SetType (Variables|Default|GetWeaponType)))

(fn SetType
  (params (WeaponType :type E_WeaponInHand%20Enum :default "NewEnumerator0"))
  (bind _skeletalmesh (Variables|Default|GetSkeletalMesh))
  (switch Utilities|FlowControl|Switch|SwitchonE_WeaponInHand WeaponType
    (:NewEnumerator1
      (Class|SkinnedMeshComponent|SetSkeletalMesh _skeletalmesh "/Game/SkeletalMeshes/Sword/SK_Blade_HeroSword10.SK_Blade_HeroSword10" true)
      (Variables|Default|SetWeaponType "NewEnumerator1"))
    (:NewEnumerator2
      (Class|SkinnedMeshComponent|SetSkeletalMesh _skeletalmesh "/Game/SkeletalMeshes/SMG11/SK_SMG11_Y.SK_SMG11_Y" true)
      (Variables|Default|SetWeaponType "NewEnumerator2"))
    (:NewEnumerator3
      (Class|SkinnedMeshComponent|SetSkeletalMesh _skeletalmesh "/Game/SkeletalMeshes/AR4/SK_AR4.SK_AR4" true)
      (Variables|Default|SetWeaponType "NewEnumerator3"))))