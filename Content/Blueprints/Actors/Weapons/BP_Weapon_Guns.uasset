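; BP_Weapon_Guns is a gun weapon actor that manages ammo in the current clip and a count of reserve clips.
; ConsumeBullets spends a round with a gunshot sound or plays an empty-clip sound, returning whether it succeeded.
; Reload refills the clip from a reserve, and PickUpClip adds reserves up to a maximum.
; Successful ammo changes push the counts to the HUD through BP_PlayerCtrl on player controller 0.
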(fn ConstructionScript
  (|CallParentFunction))

(fn ConsumeBullets
  (if (!= (Variables|Default|GetCurrentBullets) 0)
    (Math|Integer|DecrementInt (Variables|Default|GetCurrentBullets)
      (:%20%20
        (Audio|PlaySoundatLocation (Variables|Default|GetGunSound) (Transformation|GetActorLocation self) "0, 0, 0" 1.0 1.0 0.0 0 0 0)
        (CallFunction|UpdateHUD)
        (return true)))
    (else
      (Audio|PlaySoundatLocation (Variables|Default|GetEmptyClip) (Transformation|GetActorLocation self) "0, 0, 0" 1.0 1.0 0.0 0 0 0)
      (return false))))

(fn Reload
  (if (!= (Variables|Default|GetReserveClips) 0)
    (Variables|Default|SetCurrentBullets (Variables|Default|GetClipSize))
    (Math|Integer|DecrementInt (Variables|Default|GetReserveClips)
      (:%20%20
        (CallFunction|UpdateHUD)
        (return true)))
    (else
      (return false))))

(fn PickUpClip
  (if (< (Variables|Default|GetReserveClips) (Variables|Default|GetMaxClips))
    (Math|Integer|IncrementInt (Variables|Default|GetReserveClips)
      (:%20%20
        (CallFunction|UpdateHUD)))))

(fn UpdateHUD
  (bind _asbp_player_ctrl (Utilities|Casting|CastToBP_PlayerCtrl (Game|GetPlayerController 0)))
  (Default|GunHUD _asbp_player_ctrl (Utilities|Struct|MakeF_GunData (Variables|Default|GetCurrentBullets) (Variables|Default|GetClipSize) (Variables|Default|GetReserveClips))))