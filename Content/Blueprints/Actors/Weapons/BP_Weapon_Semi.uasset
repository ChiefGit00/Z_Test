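; BP_Weapon_Semi is a weapon Blueprint whose Attack fires a single hitscan shot that damages zombies.
; When attack is requested and ConsumeBullets succeeds, it line traces on the Camera channel, ignoring the player pawn, treating the End input as a direction to scale from Start.
; Only hits that cast to BP_Zombie receive a fixed amount of damage.
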(fn ConstructionScript
  (|CallParentFunction))

(fn Attack
  (params (bAttack :type Boolean) (Start :type Vector :default "0, 0, 0") (End :type Vector :default "0, 0, 0"))
  (if bAttack
    (bind _bfired (CallFunction|ConsumeBullets))
    (if _bfired
      (bind _outhit (Collision|LineTraceByChannel Start (+ Start (* End 2000)) "TraceTypeQuery2" false (Utilities|Array|MakeArray (Game|Player|GetPlayerPawn 0)) "None"))
      (bind _asbp_zombie (Utilities|Casting|CastToBP_Zombie (.hitactor _outhit)))
      (Game|Damage|ApplyDamage _asbp_zombie 25.0 0 0))))