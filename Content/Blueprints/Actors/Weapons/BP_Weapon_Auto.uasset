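; Automatic weapon Blueprint that deals hitscan damage to zombies while the attack is held.
; Attack starts or stops a looping timer that calls FireBullet, which consumes ammo before each camera-channel line trace.
; FireBullet reads Start and End from the Fire event's pins, using End as a direction.
; Hits on a zombie's Sphere component deal double the damage of other zombie hits.
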(event Custom|Fire
  (params (Start :type Vector) (End :type Vector))
  (bind _returnvalue (Utilities|Time|SetTimerbyEvent (delegate Custom|FireBullet) 0.2 true)))

(event Custom|FireBullet
  (bind _bfired (CallFunction|ConsumeBullets))
  (if _bfired
    (bind _outhit (Collision|LineTraceByChannel (stale Custom|Fire Start) (+ (stale Custom|Fire Start) (* (stale Custom|Fire End) 6000)) "TraceTypeQuery2" false (Utilities|Array|MakeArray (Game|Player|GetPlayerPawn 0)) "None"))
    (bind _asbp_zombie (Utilities|Casting|CastToBP_Zombie (.hitactor _outhit)))
    (if (== (.hitcomponent _outhit) (Variables|/Game/Blueprints/Game/BP_Zombie.BP_Zombie_C|GetSphere _asbp_zombie))
      (Game|Damage|ApplyDamage _asbp_zombie 5e+01 0 0)
      (else
        (Game|Damage|ApplyDamage _asbp_zombie 25.0 0 0)))))

(event Custom|StopFire
  (Utilities|Time|ClearandInvalidateTimerbyHandle (stale Custom|Fire _returnvalue)))

(fn ConstructionScript
  (|CallParentFunction))

(fn Attack
  (params (bAttack :type Boolean) (Start :type Vector) (End :type Vector))
  (if bAttack
    (CallFunction|Fire Start End)
    (else
      (CallFunction|StopFire))))