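; Day/night cycle actor that pitches a directional light 15 degrees per hour and refreshes a child BP_SkySphere to match.
; Once started, a looping one-second timer advances the hour while a timeline smooths rotation from the saved starting angle.
; At hour 24 it resets, pauses, and calls GM_Play's AtTwilight and, after a delay, AtDawn before resuming.
; The construction script links the sky to the light and applies the initial Time.
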(event Custom|Sun
  (bind _output_get (Variables|Default|SetTime (+ (Variables|Default|GetTime) 1.0)))
  (if (== _output_get 24.0)
    (Variables|Default|SetTime 0.0)
    (Utilities|Time|PauseTimerbyHandle (Variables|Default|GetSunTimer))
    (bind _asgm_play (Utilities|Casting|CastToGM_Play (Game|GetGameMode)))
    (Default|AtTwilight _asgm_play)
    (Utilities|FlowControl|Delay 4.0)
    (Default|AtDawn _asgm_play)
    (Utilities|Time|UnpauseTimerbyHandle (Variables|Default|GetSunTimer))
    (else
      (bind _newtrack_0 (Timeline|Timeline_0 PlayFromStart)
        (:Update
          (Transformation|SetRelativeRotation (Variables|Default|GetDirectionalLight) (Variables|Default|GetLightStartingRotation) false false)
          (Transformation|AddRelativeRotation (Variables|Default|GetDirectionalLight) (Math|Rotator|MakeRotator 0.0 (* 15 (+ (Variables|Default|GetTime) _newtrack_0)) 0.0) false false)
          (Default|RefreshMaterial (Variables|Default|GetSunSky)))))))

(event Custom|StartDynamicTime
  (bind _returnvalue (Utilities|Time|SetTimerbyEvent (delegate Custom|Sun) 1.0 true))
  (bind _output_get (Variables|Default|SetSunTimer _returnvalue)))

(event Custom|StopDynamicTime
  (Utilities|Time|PauseTimerbyHandle (stale Custom|StartDynamicTime _output_get)))

(fn ConstructionScript
  (bind _directionallight (Variables|Default|GetDirectionalLight))
  (bind _asbp_sky_sphere (Utilities|Casting|CastToBP_SkySphere (Variables|/Script/Engine.ChildActorComponent|GetChildActor (Variables|Default|GetChildActor))))
  (bind _output_get (Variables|Default|SetSunSky _asbp_sky_sphere))
  (Variables|/Game/Blueprints/Actors/BP_SkySphere.BP_SkySphere_C|SetDirectional%20light%20actor _output_get (Variables|Default|GetDirectionalLight))
  (Variables|Default|SetLightStartingRotation (Variables|/Script/Engine.SceneComponent|GetRelativeRotation _directionallight))
  (Transformation|AddRelativeRotation _directionallight (Math|Rotator|MakeRotator 0.0 (* 15 (Variables|Default|GetTime)) 0.0) false false)
  (Default|RefreshMaterial (Variables|Default|GetSunSky)))

(fn RotationOfSun
  (bind _directionallight (Variables|Default|GetDirectionalLight))
  (Transformation|SetRelativeRotation _directionallight (Variables|Default|GetLightStartingRotation) false false)
  (Transformation|AddRelativeRotation _directionallight (Math|Rotator|MakeRotator 0.0 (* 15 (Variables|Default|GetTime)) 0.0) false false)
  (Default|RefreshMaterial (Variables|Default|GetSunSky)))