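; BP_Zombie is an enemy character that chases BP_Char when it sees a pawn or survives damage, moving faster after sunset.
; A looping timer applies negative-valued damage to BP_Char while it overlaps the zombie's box.
; Incoming damage updates a world-space health bar that turns with the player's control rotation and is revealed on non-lethal hits.
; Lethal damage spawns and drops a BP_PickUp, then destroys the zombie.
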(event OnSeePawn(PawnSensing)
  (params (Pawn :type Pawn%20Object%20Reference))
  (Utilities|MovetoPawn))

(event OnComponentEndOverlap(Box)
  (params (OverlappedComponent :type Primitive%20Component%20Object%20Reference) (OtherActor :type Actor%20Object%20Reference) (OtherComp :type Primitive%20Component%20Object%20Reference) (OtherBodyIndex :type Integer))
  (Utilities|Casting|CastToBP_Char OtherActor)
  (Utilities|Time|ClearandInvalidateTimerbyHandle (stale OnComponentBeginOverlap(Box) _returnvalue)))

(event OnComponentBeginOverlap(Box)
  (params (OverlappedComponent :type Primitive%20Component%20Object%20Reference) (OtherActor :type Actor%20Object%20Reference) (OtherComp :type Primitive%20Component%20Object%20Reference) (OtherBodyIndex :type Integer) (bFromSweep :type Boolean) (SweepResult :type Hit%20Result%20Structure%20%28by%20ref%29))
  (bind _asbp_char (Utilities|Casting|CastToBP_Char OtherActor))
  (bind _returnvalue (Utilities|Time|SetTimerbyEvent (delegate Custom|DamagePawn) 0.5 true)))

(event Custom|DamagePawn
  (Game|Damage|ApplyDamage (stale OnComponentBeginOverlap(Box) _asbp_char) -15.0 0 0))

(event EventOnSunSet
  (Variables|/Script/Engine.CharacterMovementComponent|SetMaxWalkSpeed (Variables|Character|GetCharacterMovement) 2.5e+02))

(event EventTick
  (params (DeltaSeconds :type Float%20%28single-precision%29))
  (bind _returnvalue (Game|GetPlayerController 0))
  (bind _returnvalue_2 (Pawn|GetControlRotation _returnvalue :!class /Script/Engine.Controller))
  ;[1 1 1] Orient Health Widget
  (Transformation|SetWorldRotation (Variables|Default|GetWidget) (Math|Rotator|MakeRotator (.roll _returnvalue_2) (.pitch _returnvalue_2) (- (.yaw _returnvalue_2) 1.8e+02)) false false))

(event EventBeginPlay
  ;[1 1 1] Begin Play (Set Health Widget)
  (bind _aswb_zombie_health (Utilities|Casting|CastToWB_ZombieHealth (UserInterface|GetUserWidgetObject (Variables|Default|GetWidget))))
  (bind _output_get (Variables|Default|SetWB_Health _aswb_zombie_health))
  (Default|SetHealth _output_get (/ (Variables|Default|GetCurrentHealth) (Variables|Default|GetMaxHealth))))

(event Game|Damage|EventAnyDamage
  (params (Damage :type Float%20%28single-precision%29) (DamageType :type Damage%20Type%20Object%20Reference) (InstigatedBy :type Controller%20Object%20Reference) (DamageCauser :type Actor%20Object%20Reference))
  (bind _self self)
  (bind _returnvalue (Transformation|GetActorLocation _self))
  ;[1 1 1] Receive Damage
  (if (> (- (Variables|Default|GetCurrentHealth) Damage) 0.0)
    (Variables|Default|SetCurrentHealth (- (Variables|Default|GetCurrentHealth) Damage))
    (CallFunction|UpdateHealthWidget)
    (Rendering|SetVisibility (Variables|Default|GetWidget) true false)
    (Utilities|MovetoPawn)
    (else
      (Variables|Default|SetCurrentHealth 0.0)
      (CallFunction|UpdateHealthWidget)
      (bind _returnvalue_2 (Game|SpawnActorfromClass "/Game/Blueprints/Actors/Weapons/BP_PickUp.BP_PickUp_C" (Math|Transform|MakeTransform (Math|Vector|MakeVector (.x _returnvalue) (.y _returnvalue) 0.0) "0, 0, 0" "1,1,1") "Undefined" 0 0))
      (Default|Drop _returnvalue_2)
      (Actor|DestroyActor))))

(event EventOnSunRise
  (Variables|/Script/Engine.CharacterMovementComponent|SetMaxWalkSpeed (Variables|Character|GetCharacterMovement) 1e+02)
  (Components|Movement|StopMovementImmediately (Variables|Character|GetCharacterMovement)))

(fn ConstructionScript)

(fn UpdateHealthWidget
  (Progress|SetPercent (Variables|/Game/UI/WB_ZombieHealth.WB_ZombieHealth_C|GetProgressBar_Health (Variables|Default|GetWB_Health)) (/ (Variables|Default|GetCurrentHealth) (Variables|Default|GetMaxHealth))))