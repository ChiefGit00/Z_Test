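; Player character with switchable first/third-person cameras, sprint, crouch, zoom and a spotlight toggled at sunrise and sunset.
; Pickups spawn a sword, semi-auto or auto gun on body sockets; equipping moves it to the hand socket, and dropping spawns BP_PickUp.
; Gun attacks take aim data from the active camera.
; Damage, timer-driven health regen while standing still, and weapon changes are forwarded to BP_PlayerCtrl.
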(event Custom|VelocityCheck
  ;[1 1 1] Increment Health on Rest
  (Utilities|Time|SetTimerbyEvent (delegate Custom|CheckVelocity0) 1.0 true))

(event Custom|CheckVelocity0
  ;[1 1 1] Increment Health on Rest
  (if (== (Math|Vector|VectorLength (Transformation|GetVelocity)) 0.0)
    (Math|Integer|IncrementInt (Variables|Default|GetRestCount)
      (:%20%20
        (if (> (Variables|Default|GetRestCount) 2)
          (Default|UpdateHealth (Variables|Default|GetPlayerCtrl) 5.0))))
    (else
      (Variables|Default|SetRestCount 0))))

(event Game|Damage|EventAnyDamage
  (params (Damage :type Float%20%28single-precision%29) (DamageType :type Damage%20Type%20Object%20Reference) (InstigatedBy :type Controller%20Object%20Reference) (DamageCauser :type Actor%20Object%20Reference))
  ;[1 1 1] Damage
  (Default|UpdateHealth (Variables|Default|GetPlayerCtrl) Damage)
  (Variables|Default|SetRestCount 0)
  (Audio|SpawnSoundatLocation "/Game/Sounds/PlayerHit.PlayerHit" (Transformation|GetActorLocation self) "0, 0, 0" 1.0 1.0 0.0 0 0))

(event EventPossessed
  (params (NewController :type Controller%20Object%20Reference))
  ;[1 1 1] Possession
  (bind _asbp_player_ctrl (Utilities|Casting|CastToBP_PlayerCtrl NewController))
  (Variables|Default|SetPlayerCtrl _asbp_player_ctrl)
  (Components|Activation|SetActive (Variables|Default|GetCameraTP) true false)
  (Components|Activation|SetActive (Variables|Default|GetCameraFP) false false))

(event EventBeginPlay
  (CallFunction|VelocityCheck))

(event EventOnSunRise
  (Rendering|SetVisibility (Variables|Default|GetSpotLight) false false))

(event EventOnSunSet
  (Rendering|SetVisibility (Variables|Default|GetSpotLight) true false))

(event Input|ActionEvents|InputActionCamera
  (params (Key :type Key%20Structure :default "None"))
  (bind _cameratp (Variables|Default|GetCameraTP))
  (bind _camerafp (Variables|Default|GetCameraFP))
  ;[1 1 1] Input Actions
  (:Pressed
    (Utilities|FlowControl|FlipFlop
      (:A
        (Components|Activation|SetActive _cameratp false false)
        (Components|Activation|SetActive _camerafp true false)
        (Variables|Default|SetbTPS false))
      (:B
        (Components|Activation|SetActive _cameratp true false)
        (Components|Activation|SetActive _camerafp false false)
        (Variables|Default|SetbTPS true)))))

(event Input|ActionEvents|InputActionJump
  (params (Key :type Key%20Structure :default "None"))
  ;[1 1 1] Input Actions
  (:Pressed
    (Character|Jump)))

(event Input|ActionEvents|InputActionDrop
  (params (Key :type Key%20Structure :default "None"))
  ;[1 1 1] ThrowWeapon
  (:Pressed
    (CallFunction|ThrowWeapon)))

(event Input|ActionEvents|InputActionRun
  (params (Key :type Key%20Structure :default "None"))
  ;[1 1 1] Run
  (:Pressed
    (if (Variables|Default|GetbIsCrouched)
      (Character|UnCrouch))
    (Variables|/Script/Engine.CharacterMovementComponent|SetMaxWalkSpeed (Variables|Character|GetCharacterMovement) 1.2e+03)
    (if (Variables|Default|GetbTPS)
      (Variables|/Script/Engine.SpringArmComponent|SetTargetArmLength (Variables|Default|GetSpringArmTP) 3.5e+02)))
  (:Released
    (Variables|/Script/Engine.CharacterMovementComponent|SetMaxWalkSpeed (Variables|Character|GetCharacterMovement) 6e+02)
    (if (Variables|Default|GetbTPS)
      (Variables|/Script/Engine.SpringArmComponent|SetTargetArmLength (Variables|Default|GetSpringArmTP) 3e+02))))

(event Input|ActionEvents|InputActionReload
  (params (Key :type Key%20Structure :default "None"))
  (bind _semi (Variables|Default|GetSemi))
  (bind _auto (Variables|Default|GetAuto))
  ;[1 1 1] Reload
  (:Pressed
    (switch Utilities|FlowControl|Switch|SwitchonE_WeaponInHand (Variables|Default|GetCurrentWeapon)
      (:NewEnumerator2
        (if (> (Variables|/Game/Blueprints/Actors/Weapons/BP_Weapon_Guns.BP_Weapon_Guns_C|GetReserveClips _semi) 0)
          (Variables|Default|SetbReloading true)
          (Utilities|FlowControl|Delay 1.5)
          (Variables|Default|SetbReloading false)
          (Default|Reload _semi)))
      (:NewEnumerator3
        (if (> (Variables|/Game/Blueprints/Actors/Weapons/BP_Weapon_Guns.BP_Weapon_Guns_C|GetReserveClips _auto) 0)
          (Variables|Default|SetbReloading true)
          (Utilities|FlowControl|Delay 1.5)
          (Variables|Default|SetbReloading false)
          (Default|Reload _auto))))))

(event Input|ActionEvents|InputActionCrouch
  (params (Key :type Key%20Structure :default "None"))
  ;[1 1 1] Input Actions
  (:Pressed
    (Utilities|FlowControl|FlipFlop
      (:A
        (Character|Crouch))
      (:B
        (Character|UnCrouch)))))

(event Input|ActionEvents|InputActionZoom
  (params (Key :type Key%20Structure :default "None"))
  (bind _btps (Variables|Default|GetbTPS))
  ;[1 1 1] Zoom
  (:Pressed
    (if _btps
      (Variables|/Script/Engine.CameraComponent|SetFieldOfView (Variables|Default|GetCameraTP) 5e+01)
      (else
        (Variables|/Script/Engine.CameraComponent|SetFieldOfView (Variables|Default|GetCameraFP) 5e+01))))
  (:Released
    (if _btps
      (Variables|/Script/Engine.CameraComponent|SetFieldOfView (Variables|Default|GetCameraTP) 9e+01)
      (else
        (Variables|/Script/Engine.CameraComponent|SetFieldOfView (Variables|Default|GetCameraFP) 9e+01)))))

(event Input|ActionEvents|InputActionAttack
  (params (Key :type Key%20Structure :default "None"))
  ;[1 1 1] Attack and Interact
  (:Pressed
    (if (not (Variables|Default|GetbReloading))
      (Variables|Default|SetbAttack true)
      (switch Utilities|FlowControl|Switch|SwitchonE_WeaponInHand (Variables|Default|GetCurrentWeapon)
        (:NewEnumerator1
          (Variables|/Game/Blueprints/Actors/Weapons/BP_Weapon_Sword.BP_Weapon_Sword_C|SetbCanAttack (Variables|Default|GetSword) true))
        (:NewEnumerator2
          (bind (_start _end) (CallFunction|GetCameraData))
          (Default|Attack (Variables|Default|GetSemi) true _start _end))
        (:NewEnumerator3
          (bind (_start_2 _end_2) (CallFunction|GetCameraData))
          (Default|Attack (Variables|Default|GetAuto) true _start_2 _end_2)))))
  (:Released
    (Variables|Default|SetbAttack false)
    (switch Utilities|FlowControl|Switch|SwitchonE_WeaponInHand (Variables|Default|GetCurrentWeapon)
      (:NewEnumerator1
        (Variables|/Game/Blueprints/Actors/Weapons/BP_Weapon_Sword.BP_Weapon_Sword_C|SetbCanAttack (Variables|Default|GetSword) false))
      (:NewEnumerator2
        (Default|Attack (Variables|Default|GetSemi) false "0, 0, 0" "0, 0, 0"))
      (:NewEnumerator3
        (Default|Attack (Variables|Default|GetAuto) false "0, 0, 0" "0, 0, 0")))))

(event Input|ActionEvents|InputActionInteract
  (params (Key :type Key%20Structure :default "None"))
  ;[1 1 1] Attack and Interact
  (:Pressed
    (Variables|Default|SetbInteract true))
  (:Released
    (Variables|Default|SetbInteract false)))

(event Input|ActionEvents|InputActionMelee
  (params (Key :type Key%20Structure :default "None"))
  ;[1 1 1] Equip
  (:Pressed
    (CallFunction|EquipWeapon "NewEnumerator1")))

(event Input|ActionEvents|InputActionSemi-Auto
  (params (Key :type Key%20Structure :default "None"))
  ;[1 1 1] Equip
  (:Pressed
    (CallFunction|EquipWeapon "NewEnumerator2")))

(event Input|ActionEvents|InputActionAuto
  (params (Key :type Key%20Structure :default "None"))
  ;[1 1 1] Equip
  (:Pressed
    (CallFunction|EquipWeapon "NewEnumerator3")))

(event Input|ActionEvents|InputAction
  (params (Key :type Key%20Structure :default "None"))
  ;[1 1 1] Equip
  (:Pressed
    (CallFunction|EquipWeapon "NewEnumerator0")))

(fn ConstructionScript)

(fn WeaponChange
  (params (NewParam :type E_WeaponInHand%20Enum :default "NewEnumerator0"))
  (switch Utilities|FlowControl|Switch|SwitchonE_WeaponInHand NewParam))

(fn PickUpWeapon
  (params (NewWeapon :type E_WeaponInHand%20Enum :default "NewEnumerator0"))
  (switch Utilities|FlowControl|Switch|SwitchonE_WeaponInHand NewWeapon
    (:NewEnumerator1
      (Utilities|IsValid (Variables|Default|GetSword)
        (:Is%20Not%20Valid
          (bind _returnvalue (Game|SpawnActorfromClass "/Game/Blueprints/Actors/Weapons/BP_Weapon_Sword.BP_Weapon_Sword_C" (Transformation|GetSocketTransform (Variables|Character|GetMesh) "Socket_Spine_02" "RTS_World") "Undefined" 0 0))
          (bind _output_get (Variables|Default|SetSword _returnvalue))
          (Transformation|AttachComponentToComponent _output_get (Variables|Character|GetMesh) "Socket_Spine_02" "SnapToTarget" "SnapToTarget" "SnapToTarget" true)
          (Utilities|Array|SetArrayElem (Variables|Default|GetEquipments) 1 (Utilities|Struct|MakeF_Equipments "NewEnumerator1" true))
          (CallFunction|EquipWeapon "NewEnumerator1"))))
    (:NewEnumerator2
      (Utilities|IsValid (Variables|Default|GetSemi)
        (:Is%20Valid
          (Default|PickUpClip (Variables|Default|GetSemi))
          (Development|PrintString "in"))
        (:Is%20Not%20Valid
          (Development|PrintString "Hello")
          (bind _returnvalue_2 (Game|SpawnActorfromClass "/Game/Blueprints/Actors/Weapons/BP_Weapon_Semi.BP_Weapon_Semi_C" (Transformation|GetSocketTransform (Variables|Character|GetMesh) "Socket_Thigh" "RTS_World") "Undefined" 0 0))
          (bind _output_get_2 (Variables|Default|SetSemi _returnvalue_2))
          (Transformation|AttachComponentToComponent _output_get_2 (Variables|Character|GetMesh) "Socket_Thigh" "SnapToTarget" "SnapToTarget" "SnapToTarget" true)
          (Utilities|Array|SetArrayElem (Variables|Default|GetEquipments) 2 (Utilities|Struct|MakeF_Equipments "NewEnumerator2" true))
          (CallFunction|EquipWeapon "NewEnumerator2"))))
    (:NewEnumerator3
      (Utilities|IsValid (Variables|Default|GetAuto)
        (:Is%20Valid
          (Default|PickUpClip (Variables|Default|GetAuto)))
        (:Is%20Not%20Valid
          (bind _returnvalue_3 (Game|SpawnActorfromClass "/Game/Blueprints/Actors/Weapons/BP_Weapon_Auto.BP_Weapon_Auto_C" (Transformation|GetSocketTransform (Variables|Character|GetMesh) "Socket_Spine_01" "RTS_World") "Undefined" 0 0))
          (bind _output_get_3 (Variables|Default|SetAuto _returnvalue_3))
          (Transformation|AttachComponentToComponent _output_get_3 (Variables|Character|GetMesh) "Socket_Spine_01" "SnapToTarget" "SnapToTarget" "SnapToTarget" true)
          (Utilities|Array|SetArrayElem (Variables|Default|GetEquipments) 3 (Utilities|Struct|MakeF_Equipments "NewEnumerator3" true))
          (CallFunction|EquipWeapon "NewEnumerator3"))))))

(fn EquipWeapon
  (params (Weapon :type E_WeaponInHand%20Enum :default "NewEnumerator0"))
  (switch Utilities|FlowControl|Switch|SwitchonE_WeaponInHand Weapon
    (:NewEnumerator0
      (if (Utilities|Enum|NotEqual(Enum) (Variables|Default|GetCurrentWeapon) "NewEnumerator0")
        (switch Utilities|FlowControl|Switch|SwitchonE_WeaponInHand (Variables|Default|GetCurrentWeapon)
          (:NewEnumerator1
            (CallFunction|UnequipWeapon "NewEnumerator1"))
          (:NewEnumerator2
            (CallFunction|UnequipWeapon "NewEnumerator2"))
          (:NewEnumerator3
            (CallFunction|UnequipWeapon "NewEnumerator3")))
        (Variables|Default|SetCurrentWeapon "NewEnumerator0")
        (Default|WeaponChange (Variables|Default|GetPlayerCtrl) "NewEnumerator0")
        (Variables|Default|SetbUseControllerRotationYaw false)))
    (:NewEnumerator1
      (if (.possess (Utilities|Array|Get(acopy) (Variables|Default|GetEquipments) 1))
        (if (Utilities|Enum|NotEqual(Enum) (Variables|Default|GetCurrentWeapon) "NewEnumerator1")
          (switch Utilities|FlowControl|Switch|SwitchonE_WeaponInHand (Variables|Default|GetCurrentWeapon)
            (:NewEnumerator0
              _)
            (:NewEnumerator1
              (CallFunction|UnequipWeapon "NewEnumerator1"))
            (:NewEnumerator2
              (CallFunction|UnequipWeapon "NewEnumerator2"))
            (:NewEnumerator3
              (CallFunction|UnequipWeapon "NewEnumerator3")))
          (Transformation|AttachComponentToComponent (Variables|Default|GetSword) (Variables|Character|GetMesh) "Socket_Weapon" "SnapToTarget" "SnapToTarget" "SnapToTarget" true)
          (bind _output_get (Variables|Default|SetCurrentWeapon "NewEnumerator1"))
          (Default|WeaponChange (Variables|Default|GetPlayerCtrl) _output_get)
          (Variables|Default|SetbUseControllerRotationYaw true))))
    (:NewEnumerator2
      (if (.possess (Utilities|Array|Get(acopy) (Variables|Default|GetEquipments) 2))
        (if (Utilities|Enum|NotEqual(Enum) (Variables|Default|GetCurrentWeapon) "NewEnumerator2")
          (switch Utilities|FlowControl|Switch|SwitchonE_WeaponInHand (Variables|Default|GetCurrentWeapon)
            (:NewEnumerator0
              _)
            (:NewEnumerator1
              (CallFunction|UnequipWeapon "NewEnumerator1"))
            (:NewEnumerator2
              (CallFunction|UnequipWeapon "NewEnumerator2"))
            (:NewEnumerator3
              (CallFunction|UnequipWeapon "NewEnumerator3")))
          (Transformation|AttachComponentToComponent (Variables|Default|GetSemi) (Variables|Character|GetMesh) "Socket_Weapon" "SnapToTarget" "SnapToTarget" "SnapToTarget" true)
          (Default|UpdateHUD (Variables|Default|GetSemi))
          (bind _output_get_2 (Variables|Default|SetCurrentWeapon "NewEnumerator2"))
          (Default|WeaponChange (Variables|Default|GetPlayerCtrl) _output_get_2)
          (Variables|Default|SetbUseControllerRotationYaw true))))
    (:NewEnumerator3
      (if (.possess (Utilities|Array|Get(acopy) (Variables|Default|GetEquipments) 3))
        (if (Utilities|Enum|NotEqual(Enum) (Variables|Default|GetCurrentWeapon) "NewEnumerator3")
          (switch Utilities|FlowControl|Switch|SwitchonE_WeaponInHand (Variables|Default|GetCurrentWeapon)
            (:NewEnumerator0
              _)
            (:NewEnumerator1
              (CallFunction|UnequipWeapon "NewEnumerator1"))
            (:NewEnumerator2
              (CallFunction|UnequipWeapon "NewEnumerator2"))
            (:NewEnumerator3
              (CallFunction|UnequipWeapon "NewEnumerator3")))
          (Transformation|AttachComponentToComponent (Variables|Default|GetAuto) (Variables|Character|GetMesh) "Socket_Weapon" "SnapToTarget" "SnapToTarget" "SnapToTarget" true)
          (Default|UpdateHUD (Variables|Default|GetAuto))
          (bind _output_get_3 (Variables|Default|SetCurrentWeapon "NewEnumerator3"))
          (Default|WeaponChange (Variables|Default|GetPlayerCtrl) _output_get_3)
          (Variables|Default|SetbUseControllerRotationYaw true))))))

(fn UnequipWeapon
  (params (Weapon :type E_WeaponInHand%20Enum :default "NewEnumerator0"))
  (switch Utilities|FlowControl|Switch|SwitchonE_WeaponInHand Weapon
    (:NewEnumerator1
      (Utilities|IsValid (Variables|Default|GetSword)
        (:Is%20Valid
          (Transformation|AttachComponentToComponent (Variables|Default|GetSword) (Variables|Character|GetMesh) "Socket_Spine_02" "SnapToTarget" "SnapToTarget" "SnapToTarget" true)
          (Variables|Default|SetCurrentWeapon "NewEnumerator0"))))
    (:NewEnumerator2
      (Utilities|IsValid (Variables|Default|GetSemi)
        (:Is%20Valid
          (Transformation|AttachComponentToComponent (Variables|Default|GetSemi) (Variables|Character|GetMesh) "Socket_Thigh" "SnapToTarget" "SnapToTarget" "SnapToTarget" true)
          (Variables|Default|SetCurrentWeapon "NewEnumerator0"))))
    (:NewEnumerator3
      (Utilities|IsValid (Variables|Default|GetAuto)
        (:Is%20Valid
          (Transformation|AttachComponentToComponent (Variables|Default|GetAuto) (Variables|Character|GetMesh) "Socket_Spine_01" "SnapToTarget" "SnapToTarget" "SnapToTarget" true)
          (Variables|Default|SetCurrentWeapon "NewEnumerator0"))))))

(fn ThrowWeapon
  (bind _returnvalue (Transformation|GetActorTransform))
  (bind _returnvalue_2 (Math|Transform|MakeTransform (Math|Vector|MakeVector (.x (.location _returnvalue)) (.y (.location _returnvalue)) 0.0)))
  (switch Utilities|FlowControl|Switch|SwitchonE_WeaponInHand (Variables|Default|GetCurrentWeapon)
    (:NewEnumerator1
      (Actor|DestroyActor (Variables|Default|GetSword))
      (Utilities|Array|SetArrayElem (Variables|Default|GetEquipments) 1 (Utilities|Struct|MakeF_Equipments "NewEnumerator1" false))
      (bind _returnvalue_3 (Game|SpawnActorfromClass "/Game/Blueprints/Actors/Weapons/BP_PickUp.BP_PickUp_C" _returnvalue_2 "Undefined" 0 0))
      (Default|SetType _returnvalue_3 "NewEnumerator1"))
    (:NewEnumerator2
      (Actor|DestroyActor (Variables|Default|GetSemi))
      (Utilities|Array|SetArrayElem (Variables|Default|GetEquipments) 2 (Utilities|Struct|MakeF_Equipments "NewEnumerator2" false))
      (bind _returnvalue_4 (Game|SpawnActorfromClass "/Game/Blueprints/Actors/Weapons/BP_PickUp.BP_PickUp_C" _returnvalue_2 "Undefined" 0 0))
      (Default|SetType _returnvalue_4 "NewEnumerator2"))
    (:NewEnumerator3
      (Actor|DestroyActor (Variables|Default|GetAuto))
      (Utilities|Array|SetArrayElem (Variables|Default|GetEquipments) 3 (Utilities|Struct|MakeF_Equipments "NewEnumerator3" false))
      (bind _returnvalue_5 (Game|SpawnActorfromClass "/Game/Blueprints/Actors/Weapons/BP_PickUp.BP_PickUp_C" _returnvalue_2 "Undefined" 0 0))
      (Default|SetType _returnvalue_5 "NewEnumerator3")))
  (CallFunction|EquipWeapon "NewEnumerator0"))

(fn GetCameraData
  (bind _cameratp (Variables|Default|GetCameraTP))
  (bind _camerafp (Variables|Default|GetCameraFP))
  (if (Variables|Default|GetbTPS)
    (return (Transformation|GetWorldLocation _cameratp) (Math|Vector|GetForwardVector _cameratp))
    (else
      (return (Transformation|GetWorldLocation _camerafp) (Math|Vector|GetForwardVector (Transformation|GetWorldRotation _camerafp))))))

(fn Reset
  (Variables|/Game/Blueprints/Game/BP_PlayerCtrl.BP_PlayerCtrl_C|SetCurrentHealth (Variables|Default|GetPlayerCtrl) 1e+02)
  (for _array_element (Utilities|Array|MakeArray (Variables|Default|GetSword) (Variables|Default|GetSemi) (Variables|Default|GetAuto))
    (Actor|DestroyActor _array_element)))