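; Experimental player character Blueprint that handles axis-driven movement and mouse look.
; Forward input switches to fast speed with orient-to-movement, while backward and sideways input switch to slow speed without it, all moving relative to control rotation.
; Mouse X yaws the controller.
; When TPS is set, mouse Y tilts the third-person spring arm within a limited pitch range; otherwise it applies inverted controller pitch.
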(event Input|AxisEvents|InputAxisForward
  (params (AxisValue :type Float%20%28single-precision%29))
  (bind _returnvalue (Pawn|GetControlRotation :!class /Script/Engine.Pawn))
  (bind _charactermovement (Variables|Character|GetCharacterMovement))
  (bind _returnvalue_2 (Math|Vector|GetForwardVector _returnvalue))
  ;[1 1 1] Walk
  ;;[1 1 1] Forward
  (if (> AxisValue 0.0)
    (Variables|/Script/Engine.CharacterMovementComponent|SetMaxWalkSpeed _charactermovement 6e+02)
    (Variables|/Script/Engine.CharacterMovementComponent|SetbOrientRotationToMovement _charactermovement true)
    (Pawn|Input|AddMovementInput _returnvalue_2 AxisValue false)
    (else
      (Pawn|Input|AddMovementInput _returnvalue_2 AxisValue false))))

(event Input|AxisEvents|InputAxisBackward
  (params (AxisValue :type Float%20%28single-precision%29))
  (bind _returnvalue (Pawn|GetControlRotation :!class /Script/Engine.Pawn))
  (bind _charactermovement (Variables|Character|GetCharacterMovement))
  (bind _returnvalue_2 (Math|Vector|GetForwardVector _returnvalue))
  ;[1 1 1] Walk
  ;;[1 1 1] Back
  (if (< AxisValue 0.0)
    (Variables|/Script/Engine.CharacterMovementComponent|SetMaxWalkSpeed _charactermovement 9e+01)
    (Variables|/Script/Engine.CharacterMovementComponent|SetbOrientRotationToMovement _charactermovement false)
    (Pawn|Input|AddMovementInput _returnvalue_2 AxisValue false)
    (else
      (Pawn|Input|AddMovementInput _returnvalue_2 AxisValue false))))

(event Input|AxisEvents|InputAxisRight
  (params (AxisValue :type Float%20%28single-precision%29))
  (bind _returnvalue (Pawn|GetControlRotation :!class /Script/Engine.Pawn))
  (bind _charactermovement (Variables|Character|GetCharacterMovement))
  (bind _returnvalue_2 (Math|Vector|GetRightVector _returnvalue))
  ;[1 1 1] Walk
  ;;[1 1 1] Walk Side
  (if (!= AxisValue 0.0)
    (Variables|/Script/Engine.CharacterMovementComponent|SetMaxWalkSpeed _charactermovement 9e+01)
    (Variables|/Script/Engine.CharacterMovementComponent|SetbOrientRotationToMovement _charactermovement false)
    (Pawn|Input|AddMovementInput _returnvalue_2 AxisValue false)
    (else
      (Pawn|Input|AddMovementInput _returnvalue_2 AxisValue false))))

(event Input|AxisEvents|InputAxisMouseX
  (params (AxisValue :type Float%20%28single-precision%29))
  ;[1 1 1] Rotation
  (Pawn|Input|AddControllerYawInput AxisValue))

(event Input|AxisEvents|InputAxisMouseY
  (params (AxisValue :type Float%20%28single-precision%29))
  (bind _springarmtp (Variables|Default|GetSpringArmTP))
  (bind _relativerotation (Variables|/Script/Engine.SceneComponent|GetRelativeRotation _springarmtp))
  (bind _returnvalue (+ AxisValue (.pitch _relativerotation)))
  ;[1 1 1] Rotation
  (if (Variables|Default|GetbTPS)
    (if (and (> _returnvalue -25.0) (< _returnvalue 25.0))
      (Transformation|AddLocalRotation (Variables|Default|GetSpringArmTP) (Math|Rotator|MakeRotator 0.0 AxisValue 0.0) false false))
    (else
      (Pawn|Input|AddControllerPitchInput (* -1 AxisValue)))))

(fn ConstructionScript
  (|CallParentFunction))