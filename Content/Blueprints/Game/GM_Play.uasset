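; GM_Play is the play game mode, handling the day/night cycle hooks and player respawn.
; On BeginPlay it starts dynamic time on BP_LightSystem.
; AtTwilight and AtDawn broadcast sunset and sunrise messages to every actor implementing I_SunAffect.
; OnDeath unpauses the game, resets BP_Char and moves the pawn to the "Start" player start, with a delay node left unwired.
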(event Custom|OnDeath
  (bind _returnvalue (Game|Player|GetPlayerPawn 0))
  (Game|SetGamePaused false)
  (bind _asbp_char (Utilities|Casting|CastToBP_Char _returnvalue))
  (Default|Reset _asbp_char)
  (Variables|Default|SetLastPlayerStart (Class|GameModeBase|FindPlayerStart 0 "Start"))
  (Transformation|SetActorLocation _returnvalue (Transformation|GetActorLocation (Variables|Default|GetLastPlayerStart)) false false))

(event EventBeginPlay
  (CallFunction|StartDay))

(fn ConstructionScript)

(fn StartDay
  (bind _returnvalue (Actor|GetActorOfClass "/Game/Blueprints/Actors/BP_LightSystem.BP_LightSystem_C"))
  (Default|StartDynamicTime _returnvalue))

(fn AtTwilight
  (bind _outactors (Actor|GetAllActorswithInterface "/Game/Blueprints/Game/I_SunAffect.I_SunAffect_C"))
  (for _array_element _outactors
    (Class|ISunAffect|OnSunSet(Message) _array_element)))

(fn AtDawn
  (bind _outactors (Actor|GetAllActorswithInterface "/Game/Blueprints/Game/I_SunAffect.I_SunAffect_C"))
  (for _array_element _outactors
    (Class|ISunAffect|OnSunRise(Message) _array_element)))