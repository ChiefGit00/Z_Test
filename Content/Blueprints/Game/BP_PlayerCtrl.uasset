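; Player controller that owns the player's health, shield, HUD and death and win screens.
; UpdateHealth clamps healing and sends negative deltas to HealthDamage, where an active shield takes the hit but grows, since the negative value is subtracted.
; Health changes call CallHealthUpdate with a normalized value, and weapon data is forwarded to the HUD.
; Death pauses the game, shows WB_Death, notifies GM_Play and calls the delayed CreateHUD.
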(event Custom|CreateHUD
  (Utilities|FlowControl|Delay 1.0)
  (Viewport|RemoveAllWidgets)
  (bind _returnvalue (UserInterface|CreateWidget "/Game/UI/WB_HUD.WB_HUD_C"))
  (bind _output_get (Variables|Default|SetHUD _returnvalue))
  (UserInterface|Viewport|AddtoViewport _output_get 0)
  (Default|CallHealthUpdate (/ (Variables|Default|GetCurrentHealth) (Variables|Default|GetMaxHealth))))

(event EventBeginPlay
  (bind _returnvalue (UserInterface|CreateWidget "/Game/UI/WB_HUD.WB_HUD_C"))
  (bind _output_get (Variables|Default|SetHUD _returnvalue))
  (UserInterface|Viewport|AddtoViewport _output_get 0)
  (Default|CallHealthUpdate (/ (Variables|Default|GetCurrentHealth) (Variables|Default|GetMaxHealth))))

(event EventPossess
  (params (PossessedPawn :type Pawn%20Object%20Reference))
  (bind _asbp_char (Utilities|Casting|CastToBP_Char PossessedPawn))
  (Variables|Default|SetPlayerPawn _asbp_char))

(fn ConstructionScript)

(fn Dead
  (Audio|PlaySound2D "/Game/Sounds/Yell+2.Yell+2" 1.0 1.0 0.0 0 0)
  (Viewport|RemoveAllWidgets)
  (Game|SetGamePaused true)
  (bind _returnvalue (UserInterface|CreateWidget "/Game/UI/WB_Death.WB_Death_C"))
  (UserInterface|Viewport|AddtoViewport _returnvalue 0)
  (bind _asgm_play (Utilities|Casting|CastToGM_Play (Game|GetGameMode)))
  (Default|OnDeath _asgm_play)
  (CallFunction|CreateHUD))

(fn HealthDamage
  (params (Damage :type Float%20%28single-precision%29))
  (if (> (Variables|Default|GetCurrentShield) 0.0)
    (if (> (Variables|Default|GetCurrentShield) Damage)
      (Variables|Default|SetCurrentShield (- (Variables|Default|GetCurrentShield) Damage))
      (else
        (Variables|Default|SetCurrentShield 0.0)))
    (elif (> (+ (Variables|Default|GetCurrentHealth) Damage) 0.0)
      (Variables|Default|SetCurrentHealth (+ (Variables|Default|GetCurrentHealth) Damage))
      (else
        (Variables|Default|SetCurrentHealth 0.0)
        (CallFunction|Dead)))))

(fn UpdateHealth
  (params (HealthDelta :type Float%20%28single-precision%29))
  (if (< HealthDelta 0.0)
    (CallFunction|HealthDamage HealthDelta)
    (Default|CallHealthUpdate (/ (Variables|Default|GetCurrentHealth) (Variables|Default|GetMaxHealth)))
    (elif (<= (+ HealthDelta (Variables|Default|GetCurrentHealth)) (Variables|Default|GetMaxHealth))
      (bind _output_get (Variables|Default|SetCurrentHealth (+ HealthDelta (Variables|Default|GetCurrentHealth))))
      (Default|CallHealthUpdate (/ _output_get (Variables|Default|GetMaxHealth)))
      (else
        (bind _output_get_2 (Variables|Default|SetCurrentHealth (Variables|Default|GetMaxHealth)))
        (Default|CallHealthUpdate (/ _output_get_2 (Variables|Default|GetMaxHealth)))))))

(fn WeaponChange
  (params (Weapon :type E_WeaponInHand%20Enum :default "NewEnumerator0"))
  (Default|WeaponChange (Variables|Default|GetHUD) Weapon))

(fn GunHUD
  (params (GunData :type F%20Gun%20Data%20Structure))
  (Default|GunHUDSet (Variables|Default|GetHUD) GunData))

(fn Win
  (Viewport|RemoveAllWidgets)
  (bind _returnvalue (UserInterface|CreateWidget "/Game/UI/WB_Win.WB_Win_C"))
  (UserInterface|Viewport|AddtoViewport _returnvalue 0))